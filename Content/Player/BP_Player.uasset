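; BP_Player is a player character Blueprint that toggles between first-person and third-person views through Enhanced Input.
; IA_SwitchView swaps the active camera, controller-yaw rotation and skeletal mesh, using a separate first-person mesh.
; IA_Move only toggles the movement component's controller-desired rotation, on when started and off when completed; this graph adds no movement input.
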(event `EnhancedInput|/Game/Player/Input/Actions/IA_SwitchView`
  (params (ActionValue :type Boolean) (ElapsedSeconds :type "Float (double-precision)") (TriggeredSeconds :type "Float (double-precision)") (InputAction :type "InputAction Object Reference" :default "/Game/Player/Input/Actions/IA_SwitchView.IA_SwitchView"))
  (:`Completed`
    (if (`ActorComponent.IsActive` (`self.ThirdPersonCamera`))
      (`ActorComponent.Activate` (`self.Camera`) false)
      (`ActorComponent.Deactivate` (`self.ThirdPersonCamera`))
      (set `self.bUseControllerRotationYaw` true)
      (`SkeletalMeshComponent.SetSkeletalMeshAsset` (`self.Mesh`) "/Game/Mixamo/CharacterFirstPerson.CharacterFirstPerson")
      (else
        (`ActorComponent.Activate` (`self.ThirdPersonCamera`) false)
        (`ActorComponent.Deactivate` (`self.Camera`))
        (set `self.bUseControllerRotationYaw` false)
        (`SkeletalMeshComponent.SetSkeletalMeshAsset` (`self.Mesh`) "/Game/Mixamo/Character.Character")))))

(event `EnhancedInput|/Game/Player/Input/Actions/IA_Move`
  (params (ActionValue :type "Vector2D Structure") (ElapsedSeconds :type "Float (double-precision)") (TriggeredSeconds :type "Float (double-precision)") (InputAction :type "InputAction Object Reference" :default "/Game/Player/Input/Actions/IA_Move.IA_Move"))
  (bind _charactermovement (`self.CharacterMovement`))
  (:`Started`
    (set `CharacterMovementComponent.bUseControllerDesiredRotation` true _charactermovement))
  (:`Completed`
    (set `CharacterMovementComponent.bUseControllerDesiredRotation` false _charactermovement)))

(fn `UserConstructionScript`)